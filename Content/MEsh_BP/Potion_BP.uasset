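; Potion_BP is a VR potion bottle with a removable stopper and a pouring trigger.
; When a held, detached Stopper overlaps StopperLocation, its gripping controller drops it and sockets it onto the bottle mesh.
; Tick resets LiquidTest's world rotation to zero, so the liquid stays level however the bottle tilts.
; When PouringBox overlaps a VRDial_BP actor, it sends that dial a random color through UpdateColor.
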(event OnComponentBeginOverlap(PouringBox)
  (params (OverlappedComponent :type Primitive%20Component%20Object%20Reference) (OtherActor :type Actor%20Object%20Reference) (OtherComp :type Primitive%20Component%20Object%20Reference) (OtherBodyIndex :type Integer) (bFromSweep :type Boolean) (SweepResult :type Hit%20Result%20Structure%20%28by%20ref%29))
  (bind _asvrdial_bp (Utilities|Casting|CastToVRDial_BP OtherActor))
  (Default|UpdateColor _asvrdial_bp (Math|Color|MakeColor (Math|Random|RandomFloatinRange 0.0 1.0) (Math|Random|RandomFloatinRange 0.0 1.0) (Math|Random|RandomFloatinRange 0.0 1.0))))

(event OnComponentBeginOverlap(StopperLocation)
  (params (OverlappedComponent :type Primitive%20Component%20Object%20Reference) (OtherActor :type Actor%20Object%20Reference) (OtherComp :type Primitive%20Component%20Object%20Reference) (OtherBodyIndex :type Integer) (bFromSweep :type Boolean) (SweepResult :type Hit%20Result%20Structure%20%28by%20ref%29))
  (bind _stopper (Variables|Default|Getstopper))
  (bind _stopperlocation (Variables|Default|GetStopperLocation))
  (bind _returnvalue (Transformation|GetRelativeTransform _stopperlocation))
  (if (and (== OtherComp _stopper) (!= (Transformation|GetAttachParent _stopper) (Variables|Default|GetStaticMeshComponent)))
    (bind (_holdingcontrollers _bisheld) (Class|VRGripInterface|IsHeld (Variables|Default|Getstopper)))
    (if _bisheld
      (Class|GripMotionControllerComponent|DropandSocketObject (.HoldingController (Utilities|Struct|BreakBPGripPair (Utilities|Array|Get(acopy) _holdingcontrollers))) (Class|VRExpansionFunctionLibrary|MakeTransformNetQuantize (.location _returnvalue) (.rotation _returnvalue) "1,1,1") (Variables|Default|Getstopper) (.GripID (Utilities|Struct|BreakBPGripPair (Utilities|Array|Get(acopy) _holdingcontrollers))) (Variables|Default|GetStaticMeshComponent) "None" true))))

(event EventBeginPlay)

(event Collision|EventActorBeginOverlap
  (params (OtherActor :type Actor%20Object%20Reference)))

(event EventTick
  (params (DeltaSeconds :type Float%20%28single-precision%29))
  (Transformation|SetWorldRotation (Variables|Default|Getliquid_test) "0, 0, 0" false false))

(fn ConstructionScript)